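; BP_InstancerEdit is a ProInstancer command that replaces selected instanced static mesh components with new ones of a chosen instance type.
; Execute gathers ISMs from the selection and, for each, caches its data, then spawns a replacement through InstanceFactory on the Destination actor or the original owner.
; InstanceSetup applies the cached data to the new component, then the old one is destroyed.
; An error is logged when CanExecute fails.
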(fn Execute
  (bind _executioncontext (Variables|Default|GetExecutionContext))
  (bind _destination (Variables|Placement|GetDestination))
  (bind _output (Utilities|ResolveSoftReference _destination))
  ;[0.15 0.15 0.15 0.5] Security Check
  (if (CallFunction|CanExecute)
    ;[0.15 0.15 0.15 0.5] Set Struct aliases and construct position calculator
    (LocalVariables|SetInstanceFactory (.instancefactory _executioncontext))
    (LocalVariables|SetInstanceSetup (.instancesetup _executioncontext))
    ;[0.15 0.15 0.15 0.5] Get all selected ISM
    (bind _selectedactors (CallFunction|GetSelection))
    (bind _ism_array (CallFunction|ActorArrtoISM _selectedactors))
    (bind _arrayelement (Utilities|Array|ReverseforEachLoop _ism_array)
      (:LoopBody
        ;[0.15 0.15 0.15 0.5] Cache old defaults data
        (bind _output_get (LocalVariables|SetOldISM _arrayelement))
        (bind _ism_data (CallFunction|GetISMData _output_get))
        (LocalVariables|SetCurrentData _ism_data)
        (Utilities|FlowControl|Sequence
          (:then_0
            ;[0.15 0.15 0.15 0.5] Set the actor that will contain the edited ISM
            (Utilities|IsValid _output
              (:Is%20Valid
                (LocalVariables|SetActorContainer _output))
              (:Is%20Not%20Valid
                ;;[0.15 0.15 0.15 0.5] Set Instance in the same actor
                (LocalVariables|SetActorContainer (Components|GetOwner (LocalVariables|GetOldISM))))))
          (:then_1
            ;[0.15 0.15 0.15 0.5] Instance new ISM
            (bind _sm_component (Default|SpawnSMComponent (LocalVariables|GetInstanceFactory) (LocalVariables|GetActorContainer) (CallFunction|GetISMType (Variables|Instance|GetInstance%20Type))))
            (bind _asinstanced_static_mesh_component (Utilities|Casting|CastToInstancedStaticMeshComponent _sm_component)) ; Other options were considered\nbefore doing two casts.\n\nHowever, considering that ISM/SM\nare classes that are already in memory\nthe cast ends up being almost free
            (LocalVariables|SetCurrentISM _asinstanced_static_mesh_component))
          (:then_2
            ;[0.15 0.15 0.15 0.5] Actor Component Configuration Layer
            ;;[0.15 0.15 0.15 0.5] Set Defaults
            (Default|SetDefaults (LocalVariables|GetInstanceSetup) (LocalVariables|GetCurrentData) (LocalVariables|GetCurrentISM)))
          (:then_3
            ;[0.15 0.15 0.15 0.5] Destroy old instance
            (Components|DestroyComponent (LocalVariables|GetOldISM) (Components|GetOwner (LocalVariables|GetOldISM))))))
      (:Completed
        (return true)))
    (else
      ;[0.15 0.15 0.15 0.5] Error
      (CallFunction|LogError "At least one static mesh needs to be selected")
      (return false))))