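; Instancer generator command that converts static mesh components from selected actors, optionally including attached actors, into ISM/HISM components.
; Execute groups components by mesh and slot-0 material, or remaps them by mesh alone when materials are ignored.
; Injected factory, setup and position-calculator objects create or reuse the destination actor, configure new ones, and fill one instanced component per group.
; It can destroy the source actors afterwards.
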(fn MeshestoMap
  (params (SMs :type Array%20of%20Static%20Mesh%20Component%20Object%20References))
  (for _array_element SMs
    ;[0.15 0.15 0.15 0.5] Variable declaration
    (bind _output_get (LocalVariables|SetSMComponent _array_element))
    (LocalVariables|SetSM (Variables|/Script/Engine.StaticMeshComponent|GetStaticMesh _output_get))
    (LocalVariables|SetMaterial (Rendering|Material|GetMaterial _output_get 0))
    ;[0.15 0.15 0.15 0.5] If there is no mesh skips iteration
    ;;[0.15 0.15 0.15 0.5] SM Component has a mesh
    (Utilities|IsValid (LocalVariables|GetSM)
      (:Is%20Valid
        ;[0.15 0.15 0.15 0.5] Add mesh/component to map
        ;;[0.15 0.15 0.15 0.5] Search
        (bind _value (Utilities|Map|Find (LocalVariables|GetMapSM) (Utilities|Struct|MakeF_MeshMaterialKey (LocalVariables|GetSM) (LocalVariables|GetMaterial))))
        ;;[0.15 0.15 0.15 0.5] Add Set to map
        ;;;[0.15 0.15 0.15 0.5] Prepare Set
        (Utilities|Set|Add (.smcomponent _value) (LocalVariables|GetSMComponent))
        (Utilities|Map|Add (LocalVariables|GetMapSM) (Utilities|Struct|MakeF_MeshMaterialKey (LocalVariables|GetSM) (LocalVariables|GetMaterial)) (Utilities|Struct|MakeF_SMValueSet (.smcomponent _value))))
      (:Is%20Not%20Valid
        ;;[0.15 0.15 0.15 0.5] Error log
        (CallFunction|LogError (|ErrorMessage)))))
  ;[0.15 0.15 0.15 0.5] Return Map
  (return (LocalVariables|GetMapSM)))

(fn ActorArrtoSM
  (params (ActorArray :type Array%20of%20Actor%20Object%20References))
  (for _array_element ActorArray
    ;[0.15 0.15 0.15 0.5] Append all SM Component into a single array
    (Utilities|Array|AppendArray (LocalVariables|GetSMArr) (Actor|GetComponentsByClass _array_element "/Script/Engine.StaticMeshComponent")))
  ;[0.15 0.15 0.15 0.5] Return all SM component
  (return (LocalVariables|GetSMArr)))

(fn Remap
  (params (Value :type Map%20of%20F%20Mesh%20Material%20Key%20Structures%20to%20Structs))
  (bind (_keypin _valuepin) (Utilities|Map|ForEachLoop(Map) Value)
    (:then
      ;[0.15 0.15 0.15 0.5] Find Set and join it with the old map one with same mesh
      (bind _result (Utilities|Set|Union (.smcomponent _valuepin) (.smcomponent (.Value (Utilities|Map|Find (LocalVariables|GetNewMap) (Utilities|Struct|BreakF_MeshMaterialKey _keypin))))))
      ;[0.15 0.15 0.15 0.5] Add to new map
      (Utilities|Map|Add (LocalVariables|GetNewMap) (Utilities|Struct|BreakF_MeshMaterialKey _keypin) (Utilities|Struct|MakeF_SMValueSet _result)))
    (:CompletedPin
      ;[0.15 0.15 0.15 0.5] Return map
      (return (LocalVariables|GetNewMap)))))

(fn GetSelection
  ;[0.15 0.15 0.15 0.5] Get Selected objects
  (bind _selectedactors (|CallParentFunction))
  (LocalVariables|SetSelection _selectedactors)
  (if (Variables|Selection|GetIncludeAttached)
    (Utilities|FlowControl|Sequence
      (:then_0
        ;[0.15 0.15 0.15 0.5] Append attached actors to selection array
        (for _array_element (LocalVariables|GetSelection)
          ;;[0.15 0.15 0.15 0.5] Attach each actor array to new array
          (Utilities|Array|AppendArray (LocalVariables|GetAttached%20Selection) (Actor|GetAttachedActors _array_element true true)))
        (Utilities|Array|AppendArray (LocalVariables|GetSelection) (LocalVariables|GetAttached%20Selection)))
      (:then_1
        (return (LocalVariables|GetSelection))))
    (else
      (return (LocalVariables|GetSelection)))))

(fn Execute
  (bind _executioncontext (Variables|Default|GetExecutionContext))
  ;[0.15 0.15 0.15 0.5] Security Check
  (if (CallFunction|CanExecute)
    ;[0.15 0.15 0.15 0.5] Set Struct aliases and construct position calculator
    (LocalVariables|SetInstanceFactory (.instancefactory _executioncontext))
    (LocalVariables|SetInstanceSetup (.instancesetup _executioncontext))
    (bind _returnvalue (Default|InstantiateCalculator (.poscalcfactory _executioncontext) (Variables|Placement|GetPosition)))
    (LocalVariables|SetPositionCalculator _returnvalue)
    ;[0.15 0.15 0.15 0.5] Iterate over all valid single static meshes selected
    ;;[0.15 0.15 0.15 0.5] Get map with SM and Material as key and SM Component as value
    (Utilities|FlowControl|Sequence
      (:then_0
        (bind _selectedactors (CallFunction|GetSelection)))
      (:then_1
        (bind _smselection (Conversion|ActorArrtoSM _selectedactors)))
      (:then_2
        (bind _staticmeshesmap (Conversion|MeshestoMap _smselection))
        (if (Variables|Generation|GetIgnoreMaterials)
          ;;[0.15 0.15 0.15 0.5] Create a Mesh-SMComponentSet Map
          (bind _mapsm (Conversion|Remap _staticmeshesmap))
          (bind (_keypin _valuepin) (Utilities|Map|ForEachLoop(Map) _mapsm)
            (:then
              ;;[0.15 0.15 0.15 0.5] Local Var declaration without material
              (|WithoutMaterialDeclaration _keypin (.smcomponent _valuepin)))
            (:CompletedPin
              ;[0.15 0.15 0.15 0.5] Delete mesh
              (if (Variables|Generation|GetDeleteMeshesActors) :!label _label
                (for _array_element _selectedactors
                  (Actor|DestroyActor _array_element))
                (return true)
                (else
                  (return true)))))
          (else
            (bind (_keypin_2 _valuepin_2) (Utilities|Map|ForEachLoop(Map) _staticmeshesmap)
              (:then
                ;;[0.15 0.15 0.15 0.5] Var declaration with material
                (|WithMaterialDeclaration (.staticmesh _keypin_2) (.material _keypin_2) (.smcomponent _valuepin_2)))
              (:CompletedPin
                (goto _label)))))
        ;[0.15 0.15 0.15 0.5] Spawning actor layer
        ;;[0.15 0.15 0.15 0.5] Get valid destination returns a new actor if none was selected
        (bind (_solveddestination _wasvalid) (Default|EnsureWrapper (LocalVariables|GetInstanceFactory) (|DestinationToHard_2)))
        (LocalVariables|SetActorContainer _solveddestination)
        ;[0.15 0.15 0.15 0.5] Configure destination if it was created
        (if _wasvalid
          _
          (else
            ;;[0.15 0.15 0.15 0.5] Configuration Layer
            ;;;[0.15 0.15 0.15 0.5] Name
            (Default|RenameInstance (LocalVariables|GetInstanceSetup) (LocalVariables|GetActorContainer) (Variables|Placement|GetName))
            ;;;[0.15 0.15 0.15 0.5] Get position from strategy
            (bind _position (Class|BPIPositionStrategy|GeneratePosition(Message) (LocalVariables|GetPositionCalculator) (LocalVariables|GetCurrentComponentSet)))
            ;;;[0.15 0.15 0.15 0.5] Position
            (Default|SetPosition (LocalVariables|GetInstanceSetup) (LocalVariables|GetActorContainer) _position (Variables|Placement|GetPositionOffset))
            ;;;[0.15 0.15 0.15 0.5] Outliner
            (Default|SetupOutliner (LocalVariables|GetInstanceSetup) (LocalVariables|GetActorContainer) (Variables|Placement|GetOutlinerFolder))))
        ;[0.15 0.15 0.15 0.5] Component Layer
        ;;[0.15 0.15 0.15 0.5] Create ISM/HISM
        (bind _sm_component (Default|SpawnSMComponent (LocalVariables|GetInstanceFactory) (LocalVariables|GetActorContainer) (CallFunction|GetISMType (Variables|Generation|GetInstanceType))))
        (bind _asinstanced_static_mesh_component (Utilities|Casting|CastToInstancedStaticMeshComponent _sm_component)) ; Other options were considered\nbefore doing two casts.\n\nHowever, considering that ISM/SM\nare classes that are already in memory\nthe cast ends up being almost free
        ;;[0.15 0.15 0.15 0.5] Set specific mesh
        (Default|SetMesh (LocalVariables|GetInstanceSetup) _asinstanced_static_mesh_component (LocalVariables|GetCurrentSM))
        ;;[0.15 0.15 0.15 0.5] Add single instances
        (Default|AddMeshes (LocalVariables|GetInstanceSetup) _asinstanced_static_mesh_component (LocalVariables|GetCurrentComponentSet))
        ;;[0.15 0.15 0.15 0.5] Add material
        (Default|SetMaterial (LocalVariables|GetInstanceSetup) _asinstanced_static_mesh_component (LocalVariables|GetCurrentMaterial))))
    (else
      ;[0.15 0.15 0.15 0.5] Error
      (CallFunction|LogError "At least one static mesh needs to be selected")
      (return false))))