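; Position calculator Blueprint in ProInstancer that computes the combined axis-aligned bounding box of a set of mesh components.
; GetBoundingBox seeds its min and max corners from the first component's bounds, using origin minus and plus box extent.
; It then loops over the set, growing both corners with component-wise vector min and max, and returns Max and Min.
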(fn GetBoundingBox
  (params (TargetSet :type Set%20of%20Primitive%20Component%20Object%20References))
  (bind _item (Utilities|Set|GetItemByIndex TargetSet))
  (bind (_origin _boxextent) (Collision|GetComponentBounds _item))
  ;[0.15 0.15 0.15 0.5] Initialize local vars
  (Utilities|FlowControl|Sequence
    (:then_0
      (LocalVariables|SetGlobalMax (+ _origin _boxextent)))
    (:then_1
      (LocalVariables|SetGlobalMin (- _origin _boxextent)))
    (:then_2
      (bind _valuepin (Utilities|Set|ForEachLoop(Set) TargetSet)
        (:then
          ;[0.15 0.15 0.15 0.5] Get bounding box surrounding all meshes
          (Utilities|FlowControl|Sequence
            (:then_0
              (LocalVariables|SetGlobalMax (Math|Vector|VectorComponentMax (+ (.Origin (Collision|GetComponentBounds _valuepin)) (.BoxExtent (Collision|GetComponentBounds _valuepin))) (LocalVariables|GetGlobalMax))))
            (:then_1
              (LocalVariables|SetGlobalMin (Math|Vector|VectorComponentMin (- (.Origin (Collision|GetComponentBounds _valuepin)) (.BoxExtent (Collision|GetComponentBounds _valuepin))) (LocalVariables|GetGlobalMin))))))
        (:CompletedPin
          (return (LocalVariables|GetGlobalMax) (LocalVariables|GetGlobalMin)))))))