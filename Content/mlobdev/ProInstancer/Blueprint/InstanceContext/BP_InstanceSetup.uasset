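; BP_InstanceSetup is a ProInstancer helper Blueprint that configures Instanced Static Mesh components and their actors.
; SetDefaults applies a data struct's mesh, materials, transform, mobility, collision, shadow and lighting flags, tags and culling, then adds world-space instances last.
; Everything after the mesh runs inside the material loop, with each material written to slot 0.
; Other helpers add instances from actors and set actor labels, outliner folders and transforms.
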(fn RenameInstance
  (params (ISMActor :type Actor%20Object%20Reference) (NewLabel :type String))
  (EditorScripting|ActorEditing|SetActorLabel ISMActor NewLabel true))

(fn AddMeshes
  (params (ISM :type Instanced%20Static%20Mesh%20Component%20Object%20Reference) (SMActor :type Set%20of%20Static%20Mesh%20Component%20Object%20References))
  ;[0.15 0.15 0.15 0.5] Get ISM transaform
  (bind _returnvalue (Transformation|GetWorldTransform ISM))
  (LocalVariables|SetISMTransform _returnvalue)
  ;[0.15 0.15 0.15 0.5] Calculate transform per instance
  (bind _valuepin (Utilities|Set|ForEachLoop(Set) SMActor)
    (:then
      (Components|InstancedStaticMesh|AddInstance ISM (Transformation|GetWorldTransform _valuepin) true))))

(fn AddMesheswithTransforms
  (params (ISM :type Instanced%20Static%20Mesh%20Component%20Object%20Reference) (Transforms :type Array%20of%20Transforms) (bWorldSpace :type Boolean))
  (Components|InstancedStaticMesh|AddInstances ISM Transforms false bWorldSpace true))

(fn SetupOutliner
  (params (Actor :type Actor%20Object%20Reference) (FolderName :type Name))
  (Class|Actor|SetFolderPath Actor FolderName))

(fn SetMesh
  (params (SMComponent :type Static%20Mesh%20Component%20Object%20Reference) (SM :type Static%20Mesh%20Object%20Reference))
  (bind _returnvalue (Components|StaticMesh|SetStaticMesh SMComponent SM))
  (if (not _returnvalue)
    ;[0.15 0.15 0.15 0.5] Error
    (Development|PrintString 0 "Error: Mesh could not be set into the Instance Static Mesh component" false true "(R=1.000000,G=0.025641,B=0.000000,A=1.000000)" 1e+01 "")))

(fn SetPosition
  (params (Actor :type Actor%20Object%20Reference) (Position :type Vector) (Offset :type Vector))
  (Transformation|SetActorLocation Actor (+ Position Offset) false false))

(fn SetMaterial
  (params (SMComponent :type Static%20Mesh%20Component%20Object%20Reference) (Material :type Material%20Interface%20Object%20Reference))
  (Utilities|IsValid Material
    (:Is%20Valid
      (Rendering|Material|SetMaterial SMComponent 0 Material))))

(fn SetCullingDefaults
  (params (ISM :type Instanced%20Static%20Mesh%20Component%20Object%20Reference) (StartCullDistance :type Integer) (EndCullDistance :type Integer))
  (Components|InstancedStaticMesh|SetCullDistances ISM StartCullDistance EndCullDistance))

(fn SetRenderDefaults
  (params (ISM :type Instanced%20Static%20Mesh%20Component%20Object%20Reference) (NewCastShadow :type Boolean) (bNewAffectDynamicIndirectLighting :type Boolean))
  (Rendering|SetCastShadow ISM NewCastShadow)
  (Class|PrimitiveComponent|SetAffectDynamicIndirectLighting ISM bNewAffectDynamicIndirectLighting))

(fn SetCollisionsDefaults
  (params (GenerateOverlapEvents :type Boolean) (ISM :type Instanced%20Static%20Mesh%20Component%20Object%20Reference) (CollisionProfile :type Name))
  (Variables|/Script/Engine.PrimitiveComponent|SetbGenerateOverlapEvents ISM GenerateOverlapEvents)
  (Collision|SetCollisionProfileName ISM CollisionProfile true :!class /Script/Engine.PrimitiveComponent))

(fn SetDefaults
  (params (ISM%20Data :type F%20ISM%20Data%20Structure) (ISM :type Instanced%20Static%20Mesh%20Component%20Object%20Reference))
  (LocalVariables|SetData ISM%20Data)
  (LocalVariables|SetInstancedStaticMesh ISM)
  ;[0.15 0.15 0.15 0.5] Set Mesh
  (MeshEdit|SetMesh (LocalVariables|GetInstancedStaticMesh) (Utilities|Struct|BreakF_ISMData (LocalVariables|GetData)))
  ;[0.15 0.15 0.15 0.5] Set Materials
  (for _array_element (Utilities|Struct|BreakF_ISMData (LocalVariables|GetData))
    (MeshEdit|SetMaterial (LocalVariables|GetInstancedStaticMesh) _array_element)
    ;[0.15 0.15 0.15 0.5] Set Transform
    (ISMConfig|SetLocationDefaults (LocalVariables|GetInstancedStaticMesh) (.Transform (Utilities|Struct|BreakF_ISMData (LocalVariables|GetData))) (.ComponentMobility (Utilities|Struct|BreakF_ISMData (LocalVariables|GetData))))
    ;[0.15 0.15 0.15 0.5] Set collision
    (ISMConfig|SetCollisionsDefaults (.GenerateOverlapEvents (Utilities|Struct|BreakF_ISMData (LocalVariables|GetData))) (LocalVariables|GetInstancedStaticMesh) (.CollisionProfile (Utilities|Struct|BreakF_ISMData (LocalVariables|GetData))))
    ;[0.15 0.15 0.15 0.5] Set render defaults
    (ISMConfig|SetRenderDefaults (LocalVariables|GetInstancedStaticMesh) (.CastShadow (Utilities|Struct|BreakF_ISMData (LocalVariables|GetData))) (.AffectDynamicIndirectLight (Utilities|Struct|BreakF_ISMData (LocalVariables|GetData))))
    ;[0.15 0.15 0.15 0.5] Set tags
    (Variables|/Script/Engine.ActorComponent|SetComponentTags (LocalVariables|GetInstancedStaticMesh) (Utilities|Struct|BreakF_ISMData (LocalVariables|GetData)))
    ;[0.15 0.15 0.15 0.5] Set Culling
    (ISMConfig|SetCullingDefaults (LocalVariables|GetInstancedStaticMesh) (.CullStart (Utilities|Struct|BreakF_ISMData (LocalVariables|GetData))) (.CullEnd (Utilities|Struct|BreakF_ISMData (LocalVariables|GetData))))
    ;[0.15 0.15 0.15 0.5] Instances need to be added in the end
    ;;[0.15 0.15 0.15 0.5] Add Instances
    (ISMConfig|AddMesheswithTransforms (LocalVariables|GetInstancedStaticMesh) (Utilities|Struct|BreakF_ISMData (LocalVariables|GetData)) true)))

(fn SetLocationDefaults
  (params (SMComponent :type Static%20Mesh%20Component%20Object%20Reference) (Transform :type Transform) (Mobility :type EComponentMobility%20Enum :default "Static"))
  (Transformation|SetWorldTransform SMComponent Transform false false)
  (Transformation|SetMobility SMComponent Mobility))

(fn SetTransform
  (params (Actor :type Actor%20Object%20Reference) (NewTransform :type Transform%20%28by%20ref%29))
  (Transformation|SetActorTransform Actor NewTransform))